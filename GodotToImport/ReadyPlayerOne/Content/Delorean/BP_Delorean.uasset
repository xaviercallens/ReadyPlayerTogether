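; Delorean actor that plays a construction effect when it spawns and the reverse effect when destroyed.
; BeginPlay swaps every model material to a dynamic construction material and runs a timeline scaled by ConstructionTime.
; The timeline drives opacity, green-to-dark color, rotation and scale, and updates a Ready flag at full progress.
; On finish it restores the cached materials if Ready, while Destroy reverses the timeline and then expires the actor.
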(event `self.ReceiveBeginPlay`
  (bind _returnvalue (`KismetMaterialLibrary.CreateDynamicMaterialInstance` "/Game/Delorean/MI_Construct.MI_Construct"))
  (set `self.MID_Construction` _returnvalue)
  (set `self.DefaultMaterials` (`MeshComponent.GetMaterials` (`self.Model`)))
  (`TimelineComponent.SetPlayRate` (`self.ConstructionState`) (/ 1.0 (`self.ConstructionTime`)))
  (`self.SetupMaterials` false)
  (`self.Spawn`))

(event `Spawn`
  (bind (_direction _delta) (`Timeline|ConstructionState` :!label _label)
    (:`Update`
      (bind _output_get (set `self.Delta` _delta))
      (`/Engine/EditorBlueprintResources/StandardMacros.IsValid` (`self.MID_Construction`)
        (:`Is Valid`
          (`MaterialInstanceDynamic.SetScalarParameterValue` (`self.MID_Construction`) "ObjectOpacity" (`KismetMathLibrary.MapRangeClamped` _output_get 0.0 1.0 0.5 1.0))
          (`MaterialInstanceDynamic.SetVectorParameterValue` (`self.MID_Construction`) "Color" (`KismetMathLibrary.LinearColorLerp` (struct :`R` 0.8 :`G` 4.0 :`B` 0.8 :`A` 1.0) (struct :`R` 0.01 :`G` 0.01 :`B` 0.01 :`A` 1.0) (`self.Delta`)))
          (`SceneComponent.K2_SetWorldRotation` (`self.Model`) (`KismetMathLibrary.RLerp` (struct) (struct :`Yaw` 270.0) (`self.Delta`)) false false)
          (`SceneComponent.SetRelativeScale3D` (`self.Model`) (`KismetMathLibrary.VLerp` (0.01 0.01 0.01) (2.25 2.25 2.25) (`self.Delta`)))
          (if (== (`KismetMathLibrary.Lerp` 0.0 1.0 (`self.Delta`)) 1.0)
            (`|ExecutionSequence`
              (:`then_0`
                (`/Engine/EditorBlueprintResources/StandardMacros.DoOnce` false :!label _label_2
                  (:`Completed`
                    (set `self.bReady` true))))
              (:`then_1`
                (goto _label_3 :!via `Reset`)))
            (else
              (`|ExecutionSequence`
                (:`then_0`
                  (`/Engine/EditorBlueprintResources/StandardMacros.DoOnce` false :!label _label_3
                    (:`Completed`
                      (set `self.bReady` false))))
                (:`then_1`
                  (goto _label_2 :!via `Reset`))))))))
    (:`Finished`
      (if (`self.bDestroy`)
        (`self.SetLifeSpan` 0.1)
        (elif (`self.bReady`)
          (`self.SetupMaterials` true))))))

(event `Destroy`
  (`|ExecutionSequence`
    (:`then_0`
      (goto _label :!via `Reverse`))
    (:`then_1`
      (set `self.bDestroy` true)
      (if (`self.bReady`)
        (`self.SetupMaterials` false)))))

(event `SetupMaterials`
  (params (bDefault :type Boolean))
  (if bDefault
    (for (_array_element _array_index) (`self.DefaultMaterials`)
      (`PrimitiveComponent.SetMaterial` (`self.Model`) _array_index _array_element))
    (else
      (for (_ _array_index_2) (`self.DefaultMaterials`)
        (`PrimitiveComponent.SetMaterial` (`self.Model`) _array_index_2 (`self.MID_Construction`))))))

(fn `UserConstructionScript`)